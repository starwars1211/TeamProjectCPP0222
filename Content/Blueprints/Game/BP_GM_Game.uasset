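; Game mode for a multiplayer tower-defense match with quests, spawning the main tower and market at start.
; Registers controllers on login, then spawns each player's selected class and inventory actor, retrying until GameInstance selections load because login precedes BeginPlay.
; StartQuest spawns the stage's quest and adds client quest UI.
; Game State checks set win or loss; the end-flag OnRep sends player results to clients' GameInstances and destroys the session.
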(event Custom|TrySpawnCharacter
  (params (TargetPlayerController :type Player%20Controller%20Object%20Reference) (TargetPlayerIndex :type Integer))
  ;[0 0 0] Spawn Actor :: Login -> Replicate
  ;;[1 1 1] 서버 로그인이 BeginPlay보다 빨라서 GI에서 값을 못가져옴
  (if (> (Utilities|Array|Length (Variables|Default|GetCharacterSelection)) 0)
    (RunGame|SpawnCharacter (Math|Conversions|ToTransform(Vector) (.RandomLocation (AI|Navigation|GetRandomReachablePointinRadius (Math|Vector|MakeVector 0.0 0.0 5e+02) 2e+03 0 0))) TargetPlayerController TargetPlayerIndex)
    ;;[0.3336 1 0.7227] SpawnActor >> Inventory
    (RunGame|SpawnBPInventoryData TargetPlayerController TargetPlayerIndex)
    (else
      (Utilities|FlowControl|Delay 0.1)
      (CallFunction|TrySpawnCharacter TargetPlayerController TargetPlayerIndex))))

(event Custom|Server_InitQuestUI
  ;[0 0 0] Quest
  (for _array_element (Variables|Default|GetPCArray)
    (bind _asbp_pc_sample (Utilities|Casting|CastToBP_PC_Sample _array_element))
    (Default|ClientAddQuestWidgettoHUD _asbp_pc_sample)))

(event Custom|EndGame
  ;[0 0 0] SetResult To GI
  (for _array_element (Variables|Default|GetPCArray)
    (bind _asbp_pc_sample (Utilities|Casting|CastToBP_PC_Sample _array_element))
    (bind _asbp_ps (Utilities|Casting|CastToBP_PS (Variables|/Script/Engine.Controller|GetPlayerState _asbp_pc_sample)))
    (Utilities|Array|Add (Variables|Default|GetTemp_PlayerData) (Utilities|Struct|MakeS_Player_Sample (Variables|/Game/Blueprints/Gamemode/BP_PS.BP_PS_C|GetPlayerIndex _asbp_ps) (Variables|/Game/Blueprints/Gamemode/BP_PS.BP_PS_C|GetName _asbp_ps) (Variables|/Game/Blueprints/Gamemode/BP_PS.BP_PS_C|GetLevel _asbp_ps) (Variables|/Game/Blueprints/Gamemode/BP_PS.BP_PS_C|GetJob _asbp_ps) (Variables|/Game/Blueprints/Gamemode/BP_PS.BP_PS_C|GetInventoryIndex _asbp_ps) (> (Variables|/Game/Blueprints/Gamemode/BP_PS.BP_PS_C|GetCurrent%20HP _asbp_ps) 0.0))))
  (for _array_element_2 (Variables|Default|GetPCArray)
    (bind _asbp_pc_sample_2 (Utilities|Casting|CastToBP_PC_Sample _array_element_2))
    (Default|ClientSetResulttoGI _asbp_pc_sample_2 (Variables|Result|GetbIsGameWin) (Variables|Result|GetE_Result) (Variables|Default|GetTemp_PlayerData)))
  (|DestroySession (Game|GetPlayerController 0)))

(event EventPostLogin
  (params (NewPlayer :type Player%20Controller%20Object%20Reference))
  ;[0 0 0] Spawn Actor :: Login -> Replicate
  (Utilities|Array|Add (Variables|Default|GetPCArray) NewPlayer)
  (bind _asbp_pc_sample (Utilities|Casting|CastToBP_PC_Sample NewPlayer))
  (Default|ClientSetPlayerState _asbp_pc_sample)
  (Default|ReqSetGameState _asbp_pc_sample (Utilities|Array|Length (Variables|Default|GetPCArray))))

(event EventBeginPlay
  (Init|InitReference)
  (RunGame|SpawnMainTower)
  (Market|SpawnMarket))

(fn ConstructionScript)

(fn InitReference
  (bind _asbp_gi (Utilities|Casting|CastToBP_GI (Game|GetGameInstance)))
  (bind _output_get (Variables|Reference|SetServerGIRef _asbp_gi))
  (Variables|Default|SetCharacterSelection (Variables|/Game/Blueprints/Gamemode/BP_GI.BP_GI_C|GetCharacterSelection _output_get)))

(fn InitUI
  (Actor|GetActorOfClass "/Game/Blueprints/Gamemode/BP_HUD.BP_HUD_C"))

(fn SpawnMarket
  (bind _returnvalue (Game|SpawnActorfromClass "/Game/Blueprints/Game/Market/BP_Market_Sample.BP_Market_Sample_C" (Math|Transform|MakeTransform "500.000000,0.000000,0.000000") "AdjustIfPossibleButAlwaysSpawn" "MultiplyWithRoot" 0 0))
  (Variables|Reference|SetMarketRef _returnvalue))

(fn DestroyMarket
  (Utilities|IsValid (Variables|Reference|GetMarketRef)
    (:Is%20Valid
      (Widget|RemovefromParent (Variables|/Game/Blueprints/Game/Market/BP_Market_Sample.BP_Market_Sample_C|GetUIMarketInventory (Variables|Reference|GetMarketRef)))
      (Actor|DestroyActor (Variables|Reference|GetMarketRef)))
    (:Is%20Not%20Valid
      (bind _outactors (Actor|GetAllActorsOfClass "/Game/Blueprints/Game/Market/BP_Market_Sample.BP_Market_Sample_C"))
      (for _array_element _outactors
        (bind _asbp_market_sample (Utilities|Casting|CastToBP_Market_Sample _array_element))
        (Variables|Reference|SetMarketRef _asbp_market_sample)
        (Widget|RemovefromParent (Variables|/Game/Blueprints/Game/Market/BP_Market_Sample.BP_Market_Sample_C|GetUIMarketInventory (Variables|Reference|GetMarketRef)))
        (Actor|DestroyActor (Variables|Reference|GetMarketRef))))))

(fn SpawnMainTower
  (bind _returnvalue (Game|SpawnActorfromClass "/Game/Blueprints/Game/MainTower/BP_Tower_Sample.BP_Tower_Sample_C" (Math|Transform|MakeTransform "0.000000,0.000000,250.000000") "Undefined" "MultiplyWithRoot" 0 0))
  (Variables|Reference|SetMainTower _returnvalue))

(fn SpawnCharacter
  (params (SpawnTransform :type Transform) (TargetPlayerController :type Controller%20Object%20Reference) (TargetPlayerIndex :type Integer))
  (switch int (Utilities|Array|Get(acopy) (Variables|Default|GetCharacterSelection) TargetPlayerIndex)
    (:0
      (Variables|Default|SetCharacterClass "/Character/BluePrint/Characters/TPCBase/Jobs/Warrior/BP_Warrior.BP_Warrior_C"))
    (:1
      (Variables|Default|SetCharacterClass "/Character/BluePrint/Characters/TPCBase/Jobs/Gunner/BP_Gunner.BP_Gunner_C"))
    (:2
      (Variables|Default|SetCharacterClass "/Character/BluePrint/Characters/TPCBase/Jobs/Magicion/BP_Magicion.BP_Magicion_C"))
    (:3
      (Variables|Default|SetCharacterClass "/Character/BluePrint/Characters/TPCBase/Jobs/Priest/BP_Priest.BP_Priest_C")))
  (bind _returnvalue (Game|SpawnActorfromClass (Variables|Default|GetCharacterClass) SpawnTransform "AdjustIfPossibleButAlwaysSpawn" "MultiplyWithRoot" TargetPlayerController 0))
  (Pawn|Possess TargetPlayerController _returnvalue))

(fn SpawnBPInventoryData
  (params (OwnerPC :type Player%20Controller%20Object%20Reference) (PlayerIndex :type Integer))
  ;[0.3336 1 0.7227] SpawnActor >> Inventory
  (Game|SpawnActorfromClass "/InventoryModifiedPlugin/Inventory/Blueprint/BP_InventoryData.BP_InventoryData_C" (Math|Transform|MakeTransform "0, 0, 0" "0, 0, 0" "1.000000,1.000000,1.000000") "AlwaysSpawn" "MultiplyWithRoot" OwnerPC 0 0 5000 PlayerIndex 0))

(fn StartQuest
  (params (IsRunning :type Boolean) (Stage :type Integer))
  (bind _returnvalue (Game|SpawnActorfromClass "/QuestPlugin/Quest/Quest/BP_Quest.BP_Quest_C" (Math|Transform|MakeTransform "0, 0, 0") "Undefined" "MultiplyWithRoot" 0 0))
  (bind _output_get (Variables|Reference|SetQuestRef _returnvalue))
  (if (< Stage 2)
    (Default|StartStage1 _output_get)
    (else
      (Default|StartStage2 _output_get)))
  (bind _asbp_gs (Utilities|Casting|CastToBP_GS (Game|GetGameState)))
  (Variables|/Game/Blueprints/Gamemode/BP_GS.BP_GS_C|SetbIsRunning _asbp_gs IsRunning)
  (CallFunction|ServerInitQuestUI))

(fn CheckTowerDestroyed
  (bind _asbp_gs (Utilities|Casting|CastToBP_GS (Game|GetGameState)))
  (if (Variables|/Game/Blueprints/Gamemode/BP_GS.BP_GS_C|GetbIsTowerDestroyed _asbp_gs)
    (Variables|Result|SetE_Result "NewEnumerator2")
    (Variables|Result|SetbIsGameWin false)
    (Variables|Result|SetbIsEndGame true)))

(fn CheckAllPlayerDead
  (bind _asbp_gs (Utilities|Casting|CastToBP_GS (Game|GetGameState)))
  (if (Variables|/Game/Blueprints/Gamemode/BP_GS.BP_GS_C|GetbIsAllPlayerDead _asbp_gs)
    (Variables|Result|SetE_Result "NewEnumerator1")
    (Variables|Result|SetbIsGameWin false)
    (Variables|Result|SetbIsEndGame true)))

(fn CheckMissionClear
  (bind _asbp_gs (Utilities|Casting|CastToBP_GS (Game|GetGameState)))
  (if (Variables|/Game/Blueprints/Gamemode/BP_GS.BP_GS_C|GetbAllMissionCleared _asbp_gs)
    (Variables|Result|SetE_Result "NewEnumerator3")
    (Variables|Result|SetbIsGameWin true)
    (Variables|Result|SetbIsEndGame true)))

(fn OnRepBIsEndGame
  (CallFunction|EndGame))

(fn OnRepPCArray)