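; Sample main tower Blueprint that passes the damage it receives on to the game state and can display a tower UI.
; AnyDamage calls a take-damage request, which casts to BP_GS and subtracts the damage from CurrentTowerHP, printing an error if the cast fails.
; CreateUI and an identical InitUI function each create WBP_MainTower, store its reference and add it to the viewport; neither is called within this Blueprint.
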(event Custom|CreateUI
  (bind _returnvalue (UserInterface|CreateWidget "/Game/Blueprints/Game/MainTower/WBP_MainTower.WBP_MainTower_C"))
  (bind _output_get (Variables|Default|SetUITowerRef _returnvalue))
  (UserInterface|Viewport|AddtoViewport _returnvalue 0))

(event Custom|Req_TakeDamage
  (params (Damage :type Float%20%28double-precision%29))
  (bind _asbp_gs (Utilities|Casting|CastToBP_GS (Game|GetGameState))
    (:then
      (Variables|/Game/Blueprints/Gamemode/BP_GS.BP_GS_C|SetCurrentTowerHP _asbp_gs (- (Variables|/Game/Blueprints/Gamemode/BP_GS.BP_GS_C|GetCurrentTowerHP _asbp_gs) Damage)))
    (:CastFailed
      (Development|PrintString "cast to gs fail at tower"))))

(event Game|Damage|EventAnyDamage
  (params (Damage :type Float%20%28single-precision%29) (DamageType :type Damage%20Type%20Object%20Reference) (InstigatedBy :type Controller%20Object%20Reference) (DamageCauser :type Actor%20Object%20Reference))
  (CallFunction|ReqTakeDamage Damage))

(fn ConstructionScript)

(fn InitUI
  (bind _returnvalue (UserInterface|CreateWidget "/Game/Blueprints/Game/MainTower/WBP_MainTower.WBP_MainTower_C"))
  (bind _output_get (Variables|Default|SetUITowerRef _returnvalue))
  (UserInterface|Viewport|AddtoViewport _returnvalue 0))