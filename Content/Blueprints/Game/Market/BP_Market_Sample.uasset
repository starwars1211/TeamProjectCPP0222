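; Sample market actor that runs a timed market phase and shows market UI to the player.
; On BeginPlay it creates inventory and manual widgets for player 0, and resumes game time through BP_GS once MaxMarketTime elapses.
; Sphere overlaps show or hide the manual widget only when the overlapping Character's owner is the widget's owning player.
; ManualUIVisibilitySet is an empty stub.
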(event OnComponentBeginOverlap(Sphere)
  (params (OverlappedComponent :type Primitive%20Component%20Object%20Reference) (OtherActor :type Actor%20Object%20Reference) (OtherComp :type Primitive%20Component%20Object%20Reference) (OtherBodyIndex :type Integer) (bFromSweep :type Boolean) (SweepResult :type Hit%20Result%20Structure%20%28by%20ref%29))
  ;[0 0 0] UI visibility set
  (CallFunction|ToggleManualWidget OtherActor true))

(event OnComponentEndOverlap(Sphere)
  (params (OverlappedComponent :type Primitive%20Component%20Object%20Reference) (OtherActor :type Actor%20Object%20Reference) (OtherComp :type Primitive%20Component%20Object%20Reference) (OtherBodyIndex :type Integer))
  ;[0 0 0] UI visibility set
  (CallFunction|ToggleManualWidget OtherActor false))

(event Custom|CreateUI
  (bind _returnvalue (UserInterface|CreateWidget "/Game/Blueprints/Game/Market/WBP_MarketInventory.WBP_MarketInventory_C" (Game|GetPlayerController 0)))
  (bind _output_get (Variables|Default|SetUIMarketInventory _returnvalue))
  (UserInterface|Viewport|AddtoViewport _output_get 0)
  (bind _returnvalue_2 (UserInterface|CreateWidget "/Game/Blueprints/Game/Market/WBP_MarketManual.WBP_MarketManual_C" (Game|GetPlayerController 0)))
  (bind _output_get_2 (Variables|Default|SetUIMarketManual _returnvalue_2))
  (UserInterface|Viewport|AddtoViewport _output_get_2 0))

(event Custom|Toggle%20manual%20Widget
  (params (OtherActor :type Actor%20Object%20Reference) (IsVisible :type Boolean))
  (bind _uimarketmanual (Variables|Default|GetUIMarketManual))
  ;[0 0 0] UI visibility set
  (Utilities|IsValid (Variables|Default|GetUIMarketManual)
    (:Is%20Valid
      (Utilities|Casting|CastToCharacter OtherActor)
      (if (== (Widget|GetOwningPlayer (Variables|Default|GetUIMarketManual)) (Components|GetOwner OtherActor))
        (if IsVisible
          (Widget|SetVisibility _uimarketmanual "Visible")
          (Variables|Default|SetbIsManualVisible true)
          (else
            (Widget|SetVisibility _uimarketmanual "Hidden")
            (Variables|Default|SetbIsManualVisible false)))))))

(event EventBeginPlay
  (Utilities|FlowControl|Sequence
    (:then_0
      (bind _asbp_gs (Utilities|Casting|CastToBP_GS (Game|GetGameState)))
      (Utilities|FlowControl|Delay (Variables|/Game/Blueprints/Gamemode/BP_GS.BP_GS_C|GetMaxMarketTime _asbp_gs))
      (bind _asbp_gs_2 (Utilities|Casting|CastToBP_GS (Game|GetGameState)))
      (Default|ResumeGameTime _asbp_gs_2))
    (:then_1
      (CallFunction|CreateUI))))

(fn ConstructionScript)

(fn ManualUIVisibilitySet
  (params (IsCharacter :type Actor%20Object%20Reference) (IsVisible :type Boolean)))