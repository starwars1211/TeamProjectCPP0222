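; Player controller for the game level, linking each player to character spawning, quests, market and inventory UI, and the result screen.
; Pushes GameInstance selections into the PlayerState, retrying on a delay until it is valid, and asks the GameMode to spawn the character.
; M and I toggle mutually exclusive market and inventory widgets; Z and T trigger monster-kill and end-game.
; At game end, copies outcome, quest and player data to the GameInstance and opens Result.
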(event Custom|Req_KillMonster
  (bind _asbp_gm_game (Utilities|Casting|CastToBP_GM_Game (Game|GetGameMode)))
  (bind _returnvalue (Actor|GetActorOfClass "/QuestPlugin/Quest/AI/Monster/BP_AI_Level_Monster.BP_AI_Level_Monster_C"))
  (Default|ReqKillMonster (Variables|/Game/Blueprints/Game/BP_GM_Game.BP_GM_Game_C|GetQuestRef _asbp_gm_game) _returnvalue))

(event Custom|Client_AddQuestWidgetToHUD
  (bind _asbp_hud (Utilities|Casting|CastToBP_HUD (HUD|GetHUD)))
  (Default|CreateQuestUI _asbp_hud))

(event Custom|Client_SetPlayerState
  ;[0 0 0] Init & Req Spawn Character : PlayerState 생성 후 Index를 부여해야 하므로, delay를 통해 순환로직 구성
  (bind _asbp_gi (Utilities|Casting|CastToBP_GI (Game|GetGameInstance)))
  (CallFunction|ReqRepPlayerState (Variables|/Game/Blueprints/Gamemode/BP_GI.BP_GI_C|GetPlayerIndex _asbp_gi) (Variables|/Game/Blueprints/Gamemode/BP_GI.BP_GI_C|GetPlayerName _asbp_gi) (Utilities|Array|Get(acopy) (Variables|/Game/Blueprints/Gamemode/BP_GI.BP_GI_C|GetCharacterSelection _asbp_gi) (Variables|/Game/Blueprints/Gamemode/BP_GI.BP_GI_C|GetPlayerIndex _asbp_gi)))
  (CallFunction|ReqTrySpawnCharacter (Variables|/Game/Blueprints/Gamemode/BP_GI.BP_GI_C|GetPlayerIndex _asbp_gi)))

(event Custom|Client_SetResultToGI
  (params (bIsWinGame :type Boolean) (E_Result :type E_Result%20Enum :default "NewEnumerator1") (PlayerData :type Array%20of%20S%20Player%20Sample%20Structures))
  (bind _asbp_gi (Utilities|Casting|CastToBP_GI (Game|GetGameInstance)))
  ;[0 0 0] GameResult & Description
  (Variables|/Game/Blueprints/Gamemode/BP_GI.BP_GI_C|SetbIsWinGame _asbp_gi bIsWinGame)
  (Variables|/Game/Blueprints/Gamemode/BP_GI.BP_GI_C|SetE_Result _asbp_gi E_Result)
  ;[0 0 0] Quest
  (bind _asbp_gs (Utilities|Casting|CastToBP_GS (Game|GetGameState)))
  (Variables|/Game/Blueprints/Gamemode/BP_GI.BP_GI_C|SetTotalGameTime _asbp_gi (Variables|/Game/Blueprints/Gamemode/BP_GS.BP_GS_C|GetCurrentGameTime _asbp_gs))
  (Variables|/Game/Blueprints/Gamemode/BP_GI.BP_GI_C|SetLastQuestStage _asbp_gi (Variables|/Game/Blueprints/Gamemode/BP_GS.BP_GS_C|GetCurrentQuestStage _asbp_gs))
  (Variables|/Game/Blueprints/Gamemode/BP_GI.BP_GI_C|SetMaxQuestStage _asbp_gi (Variables|/Game/Blueprints/Gamemode/BP_GS.BP_GS_C|GetMaxQuestStage _asbp_gs))
  ;[0 0 0] Player
  (Variables|/Game/Blueprints/Gamemode/BP_GI.BP_GI_C|SetPlayerData _asbp_gi PlayerData)
  (Game|OpenLevel(byName) "Result"))

(event Custom|Req_TrySpawnCharacter
  (params (TargetPlayerIndex :type Integer))
  ;[0 0 0] Init & Req Spawn Character : PlayerState 생성 후 Index를 부여해야 하므로, delay를 통해 순환로직 구성
  (bind _asbp_gm_game (Utilities|Casting|CastToBP_GM_Game (Game|GetGameMode)))
  (Default|TrySpawnCharacter _asbp_gm_game self TargetPlayerIndex))

(event Custom|Req_SetGameState
  (params (CountPlayersAlive :type Integer))
  ;[0 0 0] Init & Req Spawn Character : PlayerState 생성 후 Index를 부여해야 하므로, delay를 통해 순환로직 구성
  (bind _asbp_gs (Utilities|Casting|CastToBP_GS (Game|GetGameState)))
  (Utilities|IsValid _asbp_gs
    (:Is%20Valid
      (Variables|/Game/Blueprints/Gamemode/BP_GS.BP_GS_C|SetCountPlayersAlive _asbp_gs CountPlayersAlive))
    (:Is%20Not%20Valid
      (Utilities|FlowControl|Delay 0.1)
      (CallFunction|ReqSetGameState))))

(event Custom|Req_RepPlayerState
  (params (PlayerIndex :type Integer) (PlayerName :type String) (CharacterIndex :type Integer))
  ;[0 0 0] Init & Req Spawn Character : PlayerState 생성 후 Index를 부여해야 하므로, delay를 통해 순환로직 구성
  (Utilities|IsValid (Variables|Default|GetPlayerState)
    (:Is%20Valid
      (bind _asbp_ps (Utilities|Casting|CastToBP_PS (Variables|Default|GetPlayerState)))
      (Variables|/Game/Blueprints/Gamemode/BP_PS.BP_PS_C|SetPlayerIndex _asbp_ps PlayerIndex)
      (Variables|/Game/Blueprints/Gamemode/BP_PS.BP_PS_C|SetName _asbp_ps PlayerName)
      (Variables|/Game/Blueprints/Gamemode/BP_PS.BP_PS_C|SetJob _asbp_ps (Utilities|Enum|ByteToEnumE_Job_Sample (Math|Conversions|ToByte(Integer) CharacterIndex))))
    (:Is%20Not%20Valid
      (Utilities|FlowControl|Delay 0.1)
      (CallFunction|ClientSetPlayerState))))

(event EventBeginPlay
  (Input|SetInputModeGameOnly self false))

(event Input|KeyboardEvents|T
  (params (Key :type Key%20Structure :default "None"))
  (:Pressed
    (bind _asbp_gm_game (Utilities|Casting|CastToBP_GM_Game (Game|GetGameMode)))
    (Default|EndGame _asbp_gm_game)))

(event Input|KeyboardEvents|M
  (params (Key :type Key%20Structure :default "None"))
  (bind _self self)
  ;[0 0 0] market inventory popup
  (:Pressed
    (bind _ismanualvisibile (CallFunction|CheckMarketManualVisibility))
    (if (or _ismanualvisibile (Variables|Default|GetWBP_MarketVisible))
      ;[0.3336 1 0.7227] Toggle Market Widget >> Inventory
      (bind _output_get (Variables|Default|SetWBP_MarketVisible (not (Variables|Default|GetWBP_MarketVisible))))
      (Default|EventSetMarketVisibility (Variables|/InventoryModifiedPlugin/Inventory/Blueprint/BP_InventoryData.BP_InventoryData_C|GetWBP_MarketRef (Variables|Default|GetBP_InventoryDataRef)) _output_get)
      (if (== (Variables|Default|GetWBP_InventoryVisible) true)
        (Variables|Default|SetWBP_InventoryVisible false)
        (CallFunction|SetVisibilityOfWBPInventory false)
        (Variables|/Script/Engine.PlayerController|SetbShowMouseCursor _self true)
        (Input|SetInputModeGameandUI _self 0 "DoNotLock" true false)))))

(event Input|KeyboardEvents|I
  (params (Key :type Key%20Structure :default "None"))
  (bind _self self)
  ;[0.3336 1 0.7227] Toggle Inventory Widget >> Inventory
  (:Pressed
    (bind _output_get (Variables|Default|SetWBP_InventoryVisible (not (Variables|Default|GetWBP_InventoryVisible))))
    (CallFunction|SetVisibilityOfWBPInventory _output_get)
    (if (== (Variables|Default|GetWBP_MarketVisible) true)
      (Variables|Default|SetWBP_MarketVisible false)
      (Default|EventSetMarketVisibility (Variables|/InventoryModifiedPlugin/Inventory/Blueprint/BP_InventoryData.BP_InventoryData_C|GetWBP_MarketRef (Variables|Default|GetBP_InventoryDataRef)) false)
      (Variables|/Script/Engine.PlayerController|SetbShowMouseCursor _self true)
      (Input|SetInputModeGameandUI _self 0 "DoNotLock" true false))))

(event Input|KeyboardEvents|Z
  (params (Key :type Key%20Structure :default "None"))
  ;[1 1 1] debug kill monster
  (:Pressed
    (CallFunction|ReqKillMonster)))

(fn ConstructionScript)

(fn SetVisibilityOfWBPInventory
  (params (WBP_InventoryVisible :type Boolean))
  (Default|InventoryUIVisiblility (Variables|/InventoryModifiedPlugin/Inventory/Blueprint/BP_InventoryData.BP_InventoryData_C|GetWBP_InventoryRef (Variables|Default|GetBP_InventoryDataRef)) WBP_InventoryVisible)
  (Default|CreateInventory (Variables|/InventoryModifiedPlugin/Inventory/Blueprint/BP_InventoryData.BP_InventoryData_C|GetWBP_InventoryRef (Variables|Default|GetBP_InventoryDataRef)) (Utilities|Array|Length (Variables|/InventoryModifiedPlugin/Inventory/Blueprint/BP_InventoryData.BP_InventoryData_C|GetInventoryData (Variables|Default|GetBP_InventoryDataRef))))
  (Default|UpdateInventory (Variables|/InventoryModifiedPlugin/Inventory/Blueprint/BP_InventoryData.BP_InventoryData_C|GetWBP_InventoryRef (Variables|Default|GetBP_InventoryDataRef)) (Variables|/InventoryModifiedPlugin/Inventory/Blueprint/BP_InventoryData.BP_InventoryData_C|GetInventoryData (Variables|Default|GetBP_InventoryDataRef))))

(fn CheckMarketManualVisibility
  (Utilities|IsValid (Variables|Default|GetMarketRef)
    (:Is%20Valid
      _)
    (:Is%20Not%20Valid
      (bind _returnvalue (Actor|GetActorOfClass "/Game/Blueprints/Game/Market/BP_Market_Sample.BP_Market_Sample_C"))
      (Variables|Default|SetMarketRef _returnvalue)
      (Utilities|IsValid _returnvalue
        (:Is%20Valid
          _))))
  (return (Variables|/Game/Blueprints/Game/Market/BP_Market_Sample.BP_Market_Sample_C|GetbIsManualVisible (Variables|Default|GetMarketRef))))

(fn SetResulttoGI)