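; Player state that holds a player's name, HP, MP, stamina, XP and level, with functions to change them.
; BeginPlay copies the name from the game instance, registers itself with the game mode and tries to cache the owning character and skill points.
; Stamina drains while sprinting with acceleration and otherwise regenerates; leveling up raises and refills HP and MP.
; RepNotifies dispatch MP updates and decrement the game state's alive-player count on death changes.
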(event Custom|Req_PlayersDeadCheck
  (bind _asbp_gs (Utilities|Casting|CastToBP_GS (Game|GetGameState)))
  (Variables|/Game/Blueprints/Gamemode/BP_GS.BP_GS_C|SetCountPlayersAlive _asbp_gs (- (Variables|/Game/Blueprints/Gamemode/BP_GS.BP_GS_C|GetCountPlayersAlive _asbp_gs) 1)))

(event EventBeginPlay
  (Utilities|FlowControl|Sequence
    (:then_0
      (bind _asbp_gi (Utilities|Casting|CastToBP_GI (Game|GetGameInstance)))
      (Variables|Info|SetName (Variables|/Game/Blueprints/Gamemode/BP_GI.BP_GI_C|GetPlayerName _asbp_gi)))
    (:then_1
      (bind _asbp_gm_game (Utilities|Casting|CastToBP_GM_Game (Game|GetGameMode)))
      (bind _output_get (Variables|Default|SetGMRef _asbp_gm_game))
      (Variables|/Game/Blueprints/Game/BP_GM_Game.BP_GM_Game_C|SetPSRef _output_get self))
    (:then_2
      ;[1 0 0.03977] Init BP_TP_CharacterRef >> Character
      (bind _asbp_tp_character (Utilities|Casting|CastToBP_TP_Character (Components|GetOwner)))
      (bind _output_get_2 (Variables|Default|SetBP%20TP%20CharacterR _asbp_tp_character))
      (bind _output_get_3 (Variables|Default|SetTPC%20Skill%20Component (Variables|/Character/BluePrint/Characters/BP_TP_Character.BP_TP_Character_C|GetTPC_SkillComponent _output_get_2)))
      (Variables|Default|SetPoint (Variables|/Character/BluePrint/Characters/Skill/TPC_SkillComponent.TPC_SkillComponent_C|GetPoint _output_get_3))
      (Utilities|IsValid _output_get_2
        (:Is%20Valid
          (Development|PrintString "valid character"))
        (:Is%20Not%20Valid
          (Development|PrintString "character not valid at ps"))))))

(fn ConstructionScript)

(fn AddDamage
  (params (Damage :type Float%20%28double-precision%29))
  (bind _output_get (Variables|HP|SetCurrent%20HP (- (Variables|HP|GetCurrent%20HP) Damage)))
  (bind _output_get_2 (Variables|Default|SetbIsDead (<= _output_get 0.0)))
  (return _output_get_2))

(fn AddHP
  (params (AddHP :type Float%20%28double-precision%29))
  (Variables|HP|SetCurrent%20HP (+ (Variables|HP|GetCurrent%20HP) AddHP)))

(fn AddMaxHP
  (params (AddMaxHP :type Float%20%28double-precision%29))
  (Variables|HP|SetMax%20HP (+ (Variables|HP|GetMax%20HP) AddMaxHP)))

(fn DecreaseMP
  (params (DecreaseMP :type Float%20%28double-precision%29))
  (Variables|MP|SetCurrent%20%20MP (- (Variables|MP|GetCurrent%20%20MP) DecreaseMP)))

(fn AddMP
  (params (AddMp :type Float%20%28double-precision%29))
  (Variables|MP|SetCurrent%20%20MP (+ (Variables|MP|GetCurrent%20%20MP) AddMp)))

(fn AddMaxMP
  (params (AddMaxMP :type Float%20%28double-precision%29))
  (Variables|MP|SetMax%20MP (+ (Variables|MP|GetMax%20MP) AddMaxMP)))

(fn ChangeStamina
  (bind _bp_tp_characterr (Variables|Default|GetBP%20TP%20CharacterR))
  (if (and (Variables|/Character/BluePrint/Characters/BP_TP_Character.BP_TP_Character_C|GetIsSprint _bp_tp_characterr) (Utilities|Operators|NotEqual(!=) :A (Pawn|Components|CharacterMovement|GetCurrentAcceleration (Variables|/Script/Engine.Character|GetCharacterMovement _bp_tp_characterr))))
    (Variables|Stamina|SetCurrentStamina (Math|Float|Clamp(Float) (- (Variables|Stamina|GetCurrentStamina) (* (Utilities|Time|GetWorldDeltaSeconds) (Variables|Stamina|GetStaminaRate))) 0.0 (Variables|Stamina|GetMaxStamina)))
    (else
      (Variables|Stamina|SetCurrentStamina (Math|Float|Clamp(Float) (+ (Variables|Stamina|GetCurrentStamina) (* (Utilities|Time|GetWorldDeltaSeconds) (Variables|Stamina|GetStaminaRate))) 0.0 (Variables|Stamina|GetMaxStamina))))))

(fn OnRepCurrentMP
  (Default|CallEventDispatcherUpdateMP (Variables|MP|GetCurrent%20%20MP) 0.0))

(fn IncreaseXP
  (params (AddXP :type Float%20%28double-precision%29))
  (if (< (Variables|XP|GetCurrent%20XP) 3e+02)
    (Variables|XP|SetCurrent%20XP (+ (Variables|XP|GetCurrent%20XP) AddXP))
    (if (> (Variables|XP|GetCurrent%20XP) (Variables|XP|GetMaxXP))
      (LevelXP|IncreaseLevel 1)
      (Variables|XP|SetMaxXP (+ (Variables|XP|GetMaxXP) 5e+01))
      (Variables|XP|SetCurrent%20XP 0.0))))

(fn IncreaseLevel
  (params (AddLevel :type Integer))
  (if (>= (Variables|Level|GetMaxLevel) (Variables|Level|GetLevel))
    (Variables|Level|SetLevel (Math|Integer|Clamp(Integer) (+ (Variables|Level|GetLevel) AddLevel) 0 (Variables|Level|GetMaxLevel)))
    (HPUpdate|AddMaxHP 1e+03)
    (Variables|HP|SetCurrent%20HP (Variables|HP|GetMax%20HP))
    (MP|AddMaxMP 1e+03)
    (Variables|MP|SetCurrent%20%20MP (Variables|MP|GetMax%20MP))))

(fn OnRepBIsDead
  (CallFunction|ReqPlayersDeadCheck))