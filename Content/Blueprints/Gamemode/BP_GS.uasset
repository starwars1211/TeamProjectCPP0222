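; Game state that tracks the match's timers, tower HP, quest stages and win/lose flags, alternating market and battle phases.
; Tick advances the timers and starts battle when market time expires; clearing a stage's kill, install or boss goals ends battle.
; RepNotifies drive the flow, updating HUD widgets and BP_Quest, rechecking goals, and calling BP_GM_Game for market, quest and end-condition handling.
; Quest UI setters retry after a short delay until their widget exists.
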(event Custom|Req_StartQuest
  (params (IsRunning :type Boolean))
  ;[0 0 0] Quest
  (bind _asbp_gm_game (Utilities|Casting|CastToBP_GM_Game (Game|GetGameMode)))
  (Default|StartQuest _asbp_gm_game IsRunning (Variables|Quest|GetCurrentQuestStage))
  (CallFunction|ReqSetMonsterKillUI false (> (Variables|Quest|GetCurrentQuestStage) 1)))

(event Custom|Req_SpawnMarket
  ;[0 0 0] Market
  (bind _asbp_gm_game (Utilities|Casting|CastToBP_GM_Game (Game|GetGameMode)))
  (Default|SpawnMarket _asbp_gm_game))

(event Custom|Req_DestroyMarket
  ;[0 0 0] Market
  (bind _asbp_gm_game (Utilities|Casting|CastToBP_GM_Game (Game|GetGameMode)))
  (Default|DestroyMarket _asbp_gm_game))

(event Custom|Req_SetMonsterKillUI
  (params (InIsChecked :type Boolean) (ShowStage2 :type Boolean))
  ;[0 0 0] Quest
  (bind _returnvalue (Actor|GetActorOfClass "/QuestPlugin/Quest/Quest/BP_Quest.BP_Quest_C"))
  (Default|MonsterKillQuest _returnvalue InIsChecked ShowStage2))

(event Custom|SetUIMonsterCount
  ;[0 0 0] Quest
  (bind _asbp_hud (Utilities|Casting|CastToBP_HUD (HUD|GetHUD (Game|GetPlayerController 0))))
  (Utilities|IsValid (Variables|/Game/Blueprints/Gamemode/BP_HUD.BP_HUD_C|GetWBP_QuestRef _asbp_hud)
    (:Is%20Valid
      (Variables|/QuestPlugin/Quest/Quest/WBP_QuestUI.WBP_QuestUI_C|SetMonsterCount (Variables|/Game/Blueprints/Gamemode/BP_HUD.BP_HUD_C|GetWBP_QuestRef _asbp_hud) (Variables|Quest|GetCurrentMonsterCount)))
    (:Is%20Not%20Valid
      (Utilities|FlowControl|Delay 0.1)
      (CallFunction|SetUIMonsterCount))))

(event Custom|SetUIGold
  ;[0 0 0] Quest
  (bind _asbp_hud (Utilities|Casting|CastToBP_HUD (HUD|GetHUD (Game|GetPlayerController 0))))
  (Utilities|IsValid (Variables|/Game/Blueprints/Gamemode/BP_HUD.BP_HUD_C|GetWBP_QuestRef _asbp_hud)
    (:Is%20Valid
      (Variables|/QuestPlugin/Quest/Quest/WBP_QuestUI.WBP_QuestUI_C|SetUpdateGold (Variables|/Game/Blueprints/Gamemode/BP_HUD.BP_HUD_C|GetWBP_QuestRef _asbp_hud) (Variables|Quest|GetCurrentGold)))
    (:Is%20Not%20Valid
      (Utilities|FlowControl|Delay 0.1)
      (CallFunction|SetUIGold))))

(event Custom|SetUIInstall
  ;[0 0 0] Quest
  (bind _asbp_hud (Utilities|Casting|CastToBP_HUD (HUD|GetHUD (Game|GetPlayerController 0))))
  (Utilities|IsValid (Variables|/Game/Blueprints/Gamemode/BP_HUD.BP_HUD_C|GetWBP_QuestRef _asbp_hud)
    (:Is%20Valid
      (Variables|/QuestPlugin/Quest/Quest/WBP_QuestUI.WBP_QuestUI_C|SetInstallCount (Variables|/Game/Blueprints/Gamemode/BP_HUD.BP_HUD_C|GetWBP_QuestRef _asbp_hud) (Variables|Quest|GetCurrentInstallCount)))
    (:Is%20Not%20Valid
      (Utilities|FlowControl|Delay 0.1)
      (CallFunction|SetUIInstall))))

(event Custom|Req_InitTowerHP
  ;[0 0 0] Tower
  (Variables|Default|SetCurrentTowerHP (Variables|Default|GetMaxTowerHP)))

(event EventBeginPlay
  ;[0 0 0] Tower
  (CallFunction|ReqInitTowerHP))

(event EventTick
  (params (DeltaSeconds :type Float%20%28single-precision%29))
  ;[0 0 0] Set GameTime
  (Utilities|FlowControl|Sequence
    (:then_0
      (GameTime|SetGameTime))
    (:then_1
      (if (Variables|Run|GetbIsInBattle)
        (GameTime|SetQuestTime)
        (else
          (GameTime|SetMarketTime)
          (GameTime|ResetMarketTime))))))

(fn ConstructionScript)

(fn SetGameTime
  (Variables|GameTime|SetCurrentGameTime (+ (Variables|GameTime|GetCurrentGameTime) (Utilities|Time|GetWorldDeltaSeconds))))

(fn SetMarketTime
  (Variables|GameTime|SetCurrentMarketTime (+ (Variables|GameTime|GetCurrentMarketTime) (Utilities|Time|GetWorldDeltaSeconds))))

(fn SetQuestTime
  (if (Variables|Run|GetbIsInBattle)
    (Variables|GameTime|SetCurrentQuestTime (+ (Variables|GameTime|GetCurrentQuestTime) (Utilities|Time|GetWorldDeltaSeconds)))))

(fn ResetQuestTime
  (Variables|GameTime|SetCurrentQuestTime 0.0)
  (Variables|Run|SetbIsInBattle false))

(fn ResetMarketTime
  (if (>= (Variables|GameTime|GetCurrentMarketTime) (Variables|GameTime|GetMaxMarketTime))
    (Variables|GameTime|SetCurrentMarketTime 0.0)
    (Variables|Run|SetbIsInBattle true)
    (CallFunction|ReqDestroyMarket)))

(fn UpdateQuestState
  (params (Stage2 :type Boolean))
  (QuestState|UpdateStageCount)
  (GameTime|ResetQuestTime)
  ;[0 0 0] Next Stage :: WBP_QuestUI
  (bind _returnvalue (Actor|GetActorOfClass "/QuestPlugin/Quest/Quest/BP_Quest.BP_Quest_C"))
  (Default|MonsterKillQuest _returnvalue true Stage2))

(fn UpdateStageCount
  (Variables|Quest|SetCurrentQuestStage (+ (Variables|Quest|GetCurrentQuestStage) 1))
  (if (> (Variables|Quest|GetCurrentQuestStage) (Variables|Quest|GetMaxQuestStage))
    (Variables|Run|SetbAllMissionCleared true)))

(fn OnRepBAllMissionCleared
  (bind _asbp_gm_game (Utilities|Casting|CastToBP_GM_Game (Game|GetGameMode)))
  (Default|CheckMissionClear _asbp_gm_game))

(fn OnRepBIsTowerDestroyed
  (bind _asbp_gm_game (Utilities|Casting|CastToBP_GM_Game (Game|GetGameMode)))
  (Default|CheckTowerDestroyed _asbp_gm_game))

(fn OnRepBIsAllPlayerDead
  (bind _asbp_gm_game (Utilities|Casting|CastToBP_GM_Game (Game|GetGameMode)))
  (Default|CheckAllPlayerDead _asbp_gm_game))

(fn OnRepCurrentGameTime
  (bind _asbp_hud (Utilities|Casting|CastToBP_HUD (HUD|GetHUD (Game|GetPlayerController 0))))
  (Default|SetGameTimeText (Variables|/Game/Blueprints/Gamemode/BP_HUD.BP_HUD_C|GetUIMainRef _asbp_hud) (Variables|GameTime|GetCurrentGameTime)))

(fn OnRepCurrentMarketTime
  (bind _asbp_hud (Utilities|Casting|CastToBP_HUD (HUD|GetHUD (Game|GetPlayerController 0))))
  (Default|SetMarketTimeText (Variables|/Game/Blueprints/Gamemode/BP_HUD.BP_HUD_C|GetUIMainRef _asbp_hud) (Variables|GameTime|GetCurrentMarketTime)))

(fn OnRepCurrentQuestTime
  (bind _asbp_hud (Utilities|Casting|CastToBP_HUD (HUD|GetHUD (Game|GetPlayerController 0))))
  (Default|SetQuestTimeText (Variables|/Game/Blueprints/Gamemode/BP_HUD.BP_HUD_C|GetUIMainRef _asbp_hud) (Variables|GameTime|GetCurrentQuestTime)))

(fn OnRepCurrentQuestStage
  (bind _asbp_hud (Utilities|Casting|CastToBP_HUD (HUD|GetHUD (Game|GetPlayerController 0))))
  (Default|SetQuestStageText (Variables|/Game/Blueprints/Gamemode/BP_HUD.BP_HUD_C|GetUIMainRef _asbp_hud) (Variables|Quest|GetCurrentQuestStage)))

(fn OnRepBIsinBattle
  (bind _asbp_hud (Utilities|Casting|CastToBP_HUD (HUD|GetHUD (Game|GetPlayerController 0))))
  (if (Variables|Run|GetbIsInBattle)
    (Widget|SetVisibility (Variables|/Game/Blueprints/Game/WBP_Game_Main.WBP_Game_Main_C|GetCP_MarketTime (Variables|/Game/Blueprints/Gamemode/BP_HUD.BP_HUD_C|GetUIMainRef _asbp_hud)) "Collapsed")
    (CallFunction|ReqStartQuest true)
    (else
      (Widget|SetVisibility (Variables|/Game/Blueprints/Game/WBP_Game_Main.WBP_Game_Main_C|GetCP_MarketTime (Variables|/Game/Blueprints/Gamemode/BP_HUD.BP_HUD_C|GetUIMainRef _asbp_hud)) "Visible")
      (CallFunction|ReqSpawnMarket))))

(fn OnRepCurrentMonsterCount
  (CallFunction|SetUIMonsterCount))

(fn OnRepCurrentGold
  (CallFunction|SetUIGold))

(fn OnRepMonsterKillCount
  (CallFunction|CheckQuestCleared))

(fn OnRepCurrentInstallCount
  (CallFunction|SetUIInstall)
  (CallFunction|CheckQuestCleared))

(fn OnRepBossHP
  (CallFunction|CheckQuestCleared))

(fn CheckQuestCleared
  (if (== (Variables|Quest|GetCurrentQuestStage) 1)
    (if (>= (Variables|Quest|GetMonsterKillCount) (Variables|Quest|GetMaxMonsterCount))
      (Variables|Quest|SetbIsStageCleared true)
      ;[0 0 0] Stage 1 to 2
      (QuestState|UpdateQuestState false)
      (Variables|Quest|SetMonsterKillCount 0)
      (Variables|Quest|SetbIsStageCleared false))
    (elif (Math|Boolean|ANDBoolean (<= (Variables|Quest|GetBossHP) 0) (== (Variables|Quest|GetCurrentInstallCount) 2) (>= (Variables|Quest|GetMonsterKillCount) (Variables|Quest|GetMaxMonsterCount)))
      (Variables|Quest|SetbIsStageCleared true)
      ;[0 0 0] EndGame::Clear
      (QuestState|UpdateQuestState true)
      (Development|PrintString "Hello"))))

(fn OnRepCountPlayersAlive
  (Variables|Run|SetbIsAllPlayerDead (<= (Variables|Default|GetCountPlayersAlive) 0)))

(fn OnRepCurrentTowerHP
  (bind _asbp_hud (Utilities|Casting|CastToBP_HUD (HUD|GetHUD (Game|GetPlayerController 0))))
  (Utilities|IsValid (Variables|/Game/Blueprints/Gamemode/BP_HUD.BP_HUD_C|GetUITowerRef _asbp_hud)
    (:Is%20Valid
      (Default|UpdateHP (Variables|/Game/Blueprints/Gamemode/BP_HUD.BP_HUD_C|GetUITowerRef _asbp_hud) (Variables|Default|GetCurrentTowerHP))
      (Variables|Run|SetbIsTowerDestroyed (<= (Variables|Default|GetCurrentTowerHP) 0.0)))))